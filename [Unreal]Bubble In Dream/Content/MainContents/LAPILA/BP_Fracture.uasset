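; BP_Fracture is a breakable wall that shatters when a BP_Player with Strong set overlaps its Box trigger.
; On that overlap it destroys the intact Cube, enables physics on the Geometry Collection and applies a fixed velocity-change impulse to it.
; A DoOnce limits the wall-breaking sound to one play, while the physics calls and debug prints repeat on each qualifying overlap.
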(event `self.Box.OnComponentBeginOverlap`
  (params (OverlappedComponent :type "PrimitiveComponent Object Reference") (OtherActor :type "Actor Object Reference") (OtherComp :type "PrimitiveComponent Object Reference") (OtherBodyIndex :type Integer) (bFromSweep :type Boolean) (SweepResult :type "HitResult Structure (by ref)"))
  (bind _asbp_player (cast `/Game/MainContents/LAPILA/Test/BP_Player` OtherActor))
  (if (`/Game/MainContents/LAPILA/Test/BP_Player.Strong?` _asbp_player)
    (`ActorComponent.K2_DestroyComponent` (`self.Cube`))
    (`PrimitiveComponent.SetSimulatePhysics` (`self.GeometryCollectionComponent`) true)
    (`KismetSystemLibrary.PrintString` "인식")
    (`PrimitiveComponent.AddImpulse` (`self.GeometryCollectionComponent`) (1000.0 100.0 100.0) "None" true)
    (`KismetSystemLibrary.PrintString` "나 작동했어")
    (`/Engine/EditorBlueprintResources/StandardMacros.DoOnce` false
      (:`Completed`
        (`GameplayStatics.PlaySound2D` "/Game/_Sound/벽부서지는소리.벽부서지는소리" 1.0 1.0 0.0 null null)))))

(fn `UserConstructionScript`)