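; BP_AI is an AI character that wanders the navmesh through looping random MoveTo calls and chases pawns it spots.
; PawnSensing triggers a run animation and speed boost once via a DoOnce, while a retriggerable delay returns it to walking and wandering after sightings stop.
; SkillStop disables movement, then after a delay restores walk speed and requests wandering, without re-enabling the movement mode.
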(event `self.ReceiveBeginPlay`
  (`self.RandomLocation`))

(event `RandomLocation`
  (bind _randomlocation (`NavigationSystemV1.K2_GetRandomLocationInNavigableRadius` (`self.K2_GetActorLocation`) 1000.0 null null))
  (`|AIMoveTo` self _randomlocation null
    (:`OnSuccess`
      (`self.RandomLocation`))))

(event `CanSprintAgain`
  (goto _label :!via `Reset`))

(event `self.PawnSensing.OnSeePawn`
  (params (Pawn :type "Pawn Object Reference"))
  (`|ExecutionSequence`
    (:`then_0`
      (`/Engine/EditorBlueprintResources/StandardMacros.DoOnce` false :!label _label
        (:`Completed`
          (`SkeletalMeshComponent.PlayAnimation` (`self.Mesh`) "/Game/Characters/Mannequins/Animations/Quinn/MF_Run_Fwd.MF_Run_Fwd" true)
          (set `CharacterMovementComponent.MaxWalkSpeed` 300.0 (`self.CharacterMovement`)))))
    (:`then_1`
      (`|AIMoveTo` self (0.0 0.0 0.0) Pawn
        (:`then`
          (`KismetSystemLibrary.RetriggerableDelay` 2.0)
          (`SkeletalMeshComponent.PlayAnimation` (`self.Mesh`) "/Game/Characters/Mannequins/Animations/Quinn/MF_Walk_Fwd.MF_Walk_Fwd" true)
          (set `CharacterMovementComponent.MaxWalkSpeed` 200.0 (`self.CharacterMovement`))
          (`self.CanSprintAgain`)
          (`self.RandomLocation`))))))

(event `SkillStop`
  ;[1 1 1] STOP
  (set `CharacterMovementComponent.MaxWalkSpeed` 0.0 (`self.CharacterMovement`))
  (`CharacterMovementComponent.DisableMovement` (`self.CharacterMovement`))
  (`KismetSystemLibrary.Delay` 10.0)
  (set `CharacterMovementComponent.MaxWalkSpeed` 200.0 (`self.CharacterMovement`))
  (`self.RandomLocation`))

(fn `UserConstructionScript`)