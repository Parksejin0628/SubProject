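; BP_Noise is a noise actor that travels forward, grows as it moves, and notifies the player character on overlap.
; Each Tick moves it along its forward vector by MoveSpeed and widens its X and Y scale by SizeUp.
; Overlapping player 0's character calls HitNoiseMessage on it without destroying the noise.
; It expires after NoiseDuration, or earlier through the DeleteNoise event, which also prints a debug string.
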(event `self.ReceiveBeginPlay`
  ;[1 1 1] 수명 설정
  (`self.SetLifeSpan` (`self.Noise Duration`)))

(event `self.ReceiveActorBeginOverlap`
  (params (OtherActor :type "Actor Object Reference"))
  (if (== OtherActor (`GameplayStatics.GetPlayerCharacter` 0))
    (message `/Game/_BP/Interfaces/BPI_OverlapNoise.Hit Noise` OtherActor)))

(event `self.ReceiveTick`
  (params (DeltaSeconds :type "Float (single-precision)"))
  (`|ExecutionSequence`
    (:`then_0`
      ;[1 1 1] 소음이 앞으로 전진
      (`self.K2_SetActorLocation` (+ (`self.K2_GetActorLocation`) (* (`self.GetActorForwardVector`) (* DeltaSeconds (`self.MoveSpeed`))))))
    (:`then_1`
      ;[1 1 1] 소음이 점점 커짐
      (`self.SetActorScale3D` (+ (`self.GetActorScale3D`) (* (* DeltaSeconds (`self.SizeUp`)) (1.0 1.0 0.0)))))))

(event `/Game/_BP/Interfaces/BPI_OverlapNoise.delete Noise`
  (`self.K2_DestroyActor`)
  (`KismetSystemLibrary.PrintString` "삭제"))

(fn `UserConstructionScript`)