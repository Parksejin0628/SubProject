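; BP_NoiseGenerator is an actor that periodically fires BP_Noise actors from in front of itself.
; BeginPlay plays a sound once, and Tick uses a DoOnce reset after a delay to spawn at each cycle interval.
; Each spawn inherits the generator's rotation and scale and receives its speed, growth and duration settings.
; DeleteNoise temporarily lengthens the interval, then sets a hardcoded shorter one and prints that the stop has ended.
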(event `self.ReceiveBeginPlay`
  (`GameplayStatics.PlaySoundAtLocation` "/Game/_Sound/SQ_NoiseGenerator.SQ_NoiseGenerator" (+ (`self.K2_GetActorLocation`) (* (`self.GetActorForwardVector`) (`self.Noise Spawn Distance`))) (struct) 1.0 1.0 0.0 null null null null))

(event `self.ReceiveTick`
  (params (DeltaSeconds :type "Float (single-precision)"))
  (bind _returnvalue (`self.GetActorScale3D`))
  (`|ExecutionSequence`
    (:`then_0`
      ;[1 1 1] 일정 주기마다 BP_Noise 발사
      (`/Engine/EditorBlueprintResources/StandardMacros.DoOnce` false :!label _label
        (:`Completed`
          (bind _returnvalue_2 (`|SpawnActorFromClass` "/Game/_BP/NoiseGenerator/BP_Noise.BP_Noise_C" (`KismetMathLibrary.MakeTransform` (+ (`self.K2_GetActorLocation`) (* (`self.GetActorForwardVector`) (* _returnvalue (`self.Noise Spawn Distance`)))) (`self.K2_GetActorRotation`) _returnvalue) "Undefined" "MultiplyWithRoot" null null))
          (set `/Game/_BP/NoiseGenerator/BP_Noise.MoveSpeed` (`self.Noise Move Speed`) _returnvalue_2)
          (set `/Game/_BP/NoiseGenerator/BP_Noise.SizeUp` (`self.Noise Size Up`) _returnvalue_2)
          (set `/Game/_BP/NoiseGenerator/BP_Noise.Noise Duration` (`self.Noise Duration`) _returnvalue_2)
          (`KismetSystemLibrary.Delay` (`self.Noise Cycle Time`))
          (goto _label :!via `Reset`))))))

(event `/Game/_BP/Interfaces/BPI_OverlapNoise.delete Noise`
  (set `self.Noise Cycle Time` 5.0)
  (`KismetSystemLibrary.Delay` 5.0)
  (set `self.Noise Cycle Time` 1.0)
  (`KismetSystemLibrary.PrintString` "소음 발생 장치 중지 끝"))

(fn `UserConstructionScript`)