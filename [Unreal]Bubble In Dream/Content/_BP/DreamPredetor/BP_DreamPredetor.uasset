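; BP_DreamPredetor is a predator character that switches between moving and attacking and can be stunned.
; It starts at MoveSpeed; StartAttack halts walking and sets CanAttack through a DoOnce gate.
; EndAttack resets the gate, restores speed, clears CanAttack and sets IsEndAttack.
; OverlapEnemy sets IsStun and prints a leftover Korean debug string about redshift, with no stun handling or clearing here.
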(event `self.ReceiveBeginPlay`
  (set `CharacterMovementComponent.MaxWalkSpeed` (`self.MoveSpeed`) (`self.CharacterMovement`)))

(event `Start Attack`
  (`/Engine/EditorBlueprintResources/StandardMacros.DoOnce` false :!label _label
    (:`Completed`
      (set `CharacterMovementComponent.MaxWalkSpeed` 0.0 (`self.CharacterMovement`))
      (set `self.CanAttack` true))))

(event `End Attack`
  (`|ExecutionSequence`
    (:`then_0`
      (goto _label :!via `Reset`))
    (:`then_1`
      (set `CharacterMovementComponent.MaxWalkSpeed` (`self.MoveSpeed`) (`self.CharacterMovement`))
      (set `self.CanAttack` false)
      (set `self.IsEndAttack` true))))

(event `/Game/_BP/Interfaces/BPI_HitEnemy.OverlapEnemy`
  (`KismetSystemLibrary.PrintString` "1. 적색편이가 의미하는 것이 무엇인지 설명 \n	우주 팽창의 근거중 하나로써 적색편이는 별빛의 파장을 분석하였을때 빛의 스")
  (set `self.IsStun` true))

(fn `UserConstructionScript`)